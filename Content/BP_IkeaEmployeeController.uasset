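; AI controller for an Ikea employee that makes its pawn wander at random.
; From BeginPlay it calls Patrol in an endless five-second delay loop.
; Patrol picks a reachable navmesh point within a radius of the pawn and moves straight toward it, with pathfinding off and navigation projection on.
; Debug prints report each stage, the move result and failures to find a pawn or point.
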(event `self.ReceiveBeginPlay`
  (`KismetSystemLibrary.PrintText` "Possesed")
  (`self.Patrol` :!label _label)
  (`KismetSystemLibrary.Delay` 5.0)
  (goto _label))

(fn `Patrol`
  (locals (ControllerPawn :type "Pawn Object Reference"))
  (bind _returnvalue (`self.K2_GetPawn`))
  (`KismetSystemLibrary.PrintText` "Patrol Called")
  (bind _output_get (set `local.ControllerPawn` _returnvalue))
  (if (`KismetSystemLibrary.IsValid` _returnvalue)
    (bind (_randomlocation _returnvalue_2) (`NavigationSystemV1.K2_GetRandomReachablePointInRadius` (`self.K2_GetActorLocation` _output_get) 1000.0 null null))
    (if _returnvalue_2
      (`KismetSystemLibrary.PrintText` "Moving")
      (bind _returnvalue_3 (`self.MoveToLocation` _randomlocation -1.0 true false true true null))
      (`KismetSystemLibrary.PrintText` (`KismetTextLibrary.Conv_StringToText` (`|GetEnumeratorNameAsString` _returnvalue_3)))
      (return)
      (else
        (`KismetSystemLibrary.PrintText` "Path Not Found")))
    (else
      (`KismetSystemLibrary.PrintString` "Pawn Not Found"))))

(fn `UserConstructionScript`)
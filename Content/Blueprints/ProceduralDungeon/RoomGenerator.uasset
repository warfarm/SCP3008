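; Procedural dungeon generator actor that, on BeginPlay, spawns a start room and grows a layout from random rooms attached at open exits.
; A random stream, optionally seeded, picks exit and room; rooms whose boxes overlap are destroyed and retried recursively.
; Accepted rooms add their exits until the room count runs out, then end pieces cap remaining exits.
; A timer failsafe, cleared on completion, can reopen BaseTestMap.
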(event `Spawn Start Room`
  ;[1 1 1] Spawn Start Room
  (bind _returnvalue (`|SpawnActorFromClass` "/Game/Blueprints/ProceduralDungeon/EmptyRoom.EmptyRoom_C" (`SceneComponent.K2_GetComponentToWorld` (`self.DefaultSceneRoot`)) "AlwaysSpawn" "MultiplyWithRoot" null null))
  (`KismetArrayLibrary.Array_Append` (`self.Exits List`) (`SceneComponent.GetChildrenComponents` (`/Game/Blueprints/ProceduralDungeon/MasterRoom.Exit Folder` _returnvalue) false)))

(event `Spawn Next Room`
  (bind _stream (`self.Stream`))
  ;[1 1 1] Spawn Next Room
  (bind _output_get (set `self.Selected Exit Point` (`KismetArrayLibrary.Array_RandomFromStream` (`self.Exits List`) _stream)))
  (bind _returnvalue (`|SpawnActorFromClass` (`KismetArrayLibrary.Array_RandomFromStream` (`self.Room List`) _stream) (`KismetMathLibrary.MakeTransform` (`SceneComponent.K2_GetComponentLocation` _output_get) (`SceneComponent.K2_GetComponentRotation` _output_get)) "AlwaysSpawn" "MultiplyWithRoot" null null))
  (bind _asmaster_room (cast `/Game/Blueprints/ProceduralDungeon/MasterRoom` _returnvalue))
  (set `self.Latest Room` _asmaster_room)
  (`self.Check For Overlap`))

(event `Add Overlapping Rooms To List`
  ;[1 1 1] Check for Overlap
  (for _array_element (`SceneComponent.GetChildrenComponents` (`/Game/Blueprints/ProceduralDungeon/MasterRoom.Overlap Folder` (`self.Latest Room`)) false)
    (bind _asbox_collision (cast `BoxComponent` _array_element))
    (`KismetArrayLibrary.Array_Append` (`self.Overlap List`) (`PrimitiveComponent.GetOverlappingComponents` _asbox_collision))))

(event `Check For Overlap`
  ;[1 1 1] Delete if Overlap
  (`self.Add Overlapping Rooms To List`)
  (if (`KismetArrayLibrary.Array_IsNotEmpty` (`self.Overlap List`))
    (`KismetArrayLibrary.Array_Clear` (`self.Overlap List`))
    (`self.K2_DestroyActor` (`self.Latest Room`))
    (`self.Spawn Next Room`)
    (else
      (`KismetArrayLibrary.Array_Clear` (`self.Overlap List`))
      (set `self.Room Amount` (- (`self.Room Amount`) 1))
      (`KismetArrayLibrary.Array_RemoveItem` (`self.Exits List`) (`self.Selected Exit Point`))
      (`KismetArrayLibrary.Array_Append` (`self.Exits List`) (`SceneComponent.GetChildrenComponents` (`/Game/Blueprints/ProceduralDungeon/MasterRoom.Exit Folder` (`self.Latest Room`)) false))
      (`KismetSystemLibrary.Delay` (`self.Delay Time`))
      (if (> (`self.Room Amount`) 0)
        (`self.Spawn Next Room`)
        (else
          (`self.Close Holes`)
          (set `self.Dungeon Complete` true)
          (`KismetSystemLibrary.K2_ClearAndInvalidateTimerHandle` (`self.Timer Handle`)))))))

(event `Close Holes`
  ;[1 1 1] Close Holes
  (for _array_element (`self.Exits List`)
    (`KismetSystemLibrary.Delay` (`self.Delay Time`))
    (`|SpawnActorFromClass` "/Game/Blueprints/ProceduralDungeon/RoomEnd.RoomEnd_C" (`SceneComponent.K2_GetComponentToWorld` _array_element) "AlwaysSpawn" "MultiplyWithRoot" null null)))

(event `Start Room Timer`
  ;[1 1 1] Generation Failsafe
  (bind _returnvalue (`KismetSystemLibrary.K2_SetTimerDelegate` (delegate `Check For Dungeon Complete`)))
  (set `self.Timer Handle` _returnvalue))

(event `Check For Dungeon Complete`
  ;[1 1 1] Generation Failsafe
  (if (>= (`KismetSystemLibrary.GetGameTimeInSeconds`) (* (`self.Room Amount`) 0.2))
    (`GameplayStatics.OpenLevel` "BaseTestMap")))

(event `Set Seed`
  (bind _seed (`self.Seed`))
  (bind _stream (`self.Stream`))
  ;[1 1 1] Set Seed
  (if (== _seed -1)
    (`KismetMathLibrary.SeedRandomStream` _stream)
    (else
      (`KismetMathLibrary.SetRandomStreamSeed` _stream _seed))))

(event `self.ReceiveBeginPlay`
  (`self.Set Seed`)
  (`self.Spawn Start Room`)
  (`self.Start Room Timer`)
  (`self.Spawn Next Room`))

(fn `UserConstructionScript`)
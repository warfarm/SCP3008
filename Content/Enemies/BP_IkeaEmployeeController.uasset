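; AI controller for the Ikea employee enemy, handling patrol, idle, chase and stun behavior.
; A looping state macro either patrols to a random reachable nav point or idles, with ExitAlways and ExitSafe called around it.
; AI perception sets a chase target and repeats move-to-actor while the state is CHASE, until that target is forgotten.
; OnStun sets a flag for a retriggerable delay, then re-enters the state loop.
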(event `self.ReceiveBeginPlay`
  (`KismetSystemLibrary.PrintText` "Possesed")
  (`self.ExitAlways`)
  (`self.HandleRandomStates` :!label _label)
  (`self.ExitSafe`)
  (goto _label))

(event `self.OnStun`
  (params (duration :type "Float (single-precision)"))
  (`KismetSystemLibrary.PrintString` (`KismetStringLibrary.Concat_StrStr` "Stunned For:" (`KismetStringLibrary.Conv_DoubleToString` duration)))
  (set `self.bIsStunned` true)
  (`KismetSystemLibrary.RetriggerableDelay` duration)
  (set `self.bIsStunned` false)
  (`self.ExitAlways`)
  (goto _label))

(event `self.AIPerception.OnTargetPerceptionUpdated`
  (params (Actor :type "Actor Object Reference") (Stimulus :type "AIStimulus Structure"))
  (set `self.CurrentlyChasing` Actor)
  (bind _output_get (set `self.bIsChasing` true))
  (`self.Chase` :!label _label_2)
  (if (and (`|EnumEquality` (`self.ActorState`) "CHASE") _output_get)
    (goto _label_2)))

(event `self.AIPerception.OnTargetPerceptionForgotten`
  (params (Actor :type "Actor Object Reference"))
  (if (== Actor (`self.CurrentlyChasing`))
    (set `self.bIsChasing` false)))

(fn `Chase`
  (`self.MoveToActor` (`self.CurrentlyChasing`) -1.0 true true true null)
  (return))

(fn `Patrol`
  (locals (ControllerPawn :type "Pawn Object Reference") (`Random Location` :type "Vector Structure" :default (0.0 0.0 0.0)))
  (bind _returnvalue (`self.K2_GetPawn`))
  (`KismetSystemLibrary.PrintText` "Patrol Called")
  (bind _output_get (set `local.ControllerPawn` _returnvalue))
  (if (`KismetSystemLibrary.IsValid` _returnvalue)
    (bind _returnvalue_2 (`self.K2_GetActorLocation` _output_get))
    (bind (_randomlocation _returnvalue_3) (`NavigationSystemV1.K2_GetRandomReachablePointInRadius` _returnvalue_2 1000.0 null null))
    (set `local.Random Location` _randomlocation)
    (while (and (< (`KismetMathLibrary.Vector_Distance` _returnvalue_2 (`local.Random Location`)) 500.0) _returnvalue_3)
      (set `local.Random Location` _randomlocation))
    (bind _returnvalue_4 (`self.MoveToLocation` (`local.Random Location`) -1.0 true true true true null))
    (`KismetSystemLibrary.PrintText` (`KismetTextLibrary.Conv_StringToText` (`|GetEnumeratorNameAsString` _returnvalue_4)))
    (return)
    (else
      (`KismetSystemLibrary.PrintString` "Pawn Not Found"))))

(fn `UserConstructionScript`)